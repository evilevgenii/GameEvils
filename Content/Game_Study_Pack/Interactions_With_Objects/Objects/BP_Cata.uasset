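; BP_Cata is an interactable object that opens a ZadanieWidget screen when E is pressed within its trigger box.
; Box overlap sets an InRadius flag and creates an InteractionButtonWidget prompt, which is collapsed when the overlap ends.
; Pressing E while InRadius collapses the prompt and adds a new ZadanieWidget to the viewport.
; Overlaps are not filtered by actor, and widgets are created anew each time without being removed.
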(event OnComponentBeginOverlap(Box)
  (params (OverlappedComponent :type Primitive%20Component%20Object%20Reference) (OtherActor :type Actor%20Object%20Reference) (OtherComp :type Primitive%20Component%20Object%20Reference) (OtherBodyIndex :type Integer) (bFromSweep :type Boolean) (SweepResult :type Hit%20Result%20Structure%20%28by%20ref%29))
  (bind _returnvalue (UserInterface|CreateWidget "/Game/Game_Study_Pack/Interactions_With_Objects/InteractionButtonWidget.InteractionButtonWidget_C"))
  (UserInterface|Viewport|AddtoViewport _returnvalue 0)
  (Widget|SetVisibility _returnvalue "Visible")
  (Variables|Default|SetInRadius? true))

(event OnComponentEndOverlap(Box)
  (params (OverlappedComponent :type Primitive%20Component%20Object%20Reference) (OtherActor :type Actor%20Object%20Reference) (OtherComp :type Primitive%20Component%20Object%20Reference) (OtherBodyIndex :type Integer))
  (Widget|SetVisibility (stale OnComponentBeginOverlap(Box) _returnvalue) "Collapsed")
  (Variables|Default|SetInRadius? false))

(event EventBeginPlay)

(event Collision|EventActorBeginOverlap
  (params (OtherActor :type Actor%20Object%20Reference)))

(event EventTick
  (params (DeltaSeconds :type Float%20%28single-precision%29)))

(event Input|KeyboardEvents|E
  (params (Key :type Key%20Structure))
  (:Pressed
    (if (Variables|Default|GetInRadius?)
      (Widget|SetVisibility (stale OnComponentBeginOverlap(Box) _returnvalue) "Collapsed")
      (bind _returnvalue (UserInterface|CreateWidget "/Game/Game_Study_Pack/Interactions_With_Objects/ZadanieWidget.ZadanieWidget_C"))
      (UserInterface|Viewport|AddtoViewport _returnvalue 0))))

(fn ConstructionScript)